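; Enemy character that damages an overlapping HeroCharater and awards score to the TwinMode game mode when killed.
; Overlap starts a looping timer that applies Damage at AttacksPerSecond until the hero leaves.
; AffectHealth runs CalculateHealth; on death it ignores WorldDynamic and Pawn collision, detaches the controller and destroys the actor after a delay.
; The construction script tints the body with EnemyColor through a dynamic material instance.
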(event `self.ReceiveActorBeginOverlap`
  (params (OtherActor :type "Actor Object Reference"))
  (bind _ashero_charater (cast `/Game/Blueprints/HeroCharater` OtherActor))
  (set `self.Hero` _ashero_charater)
  (`KismetSystemLibrary.K2_SetTimer` null "Damage The Hero" (/ 1.0 (`self.AttacksPerSecond`)) true))

(event `self.ReceiveActorEndOverlap`
  (params (OtherActor :type "Actor Object Reference"))
  (if (== OtherActor (`self.Hero`))
    (`KismetSystemLibrary.K2_ClearTimer` null "Damage The Hero")))

(event `Damage The Hero`
  (`/Game/Blueprints/HeroCharater.AffectHealth` (`self.Hero`) (`self.Damage`)))

(event `/Game/Blueprints/iDamageable.AffectHealth`
  (params (Delta :type "Float (double-precision)"))
  (bind _capsulecomponent (`self.CapsuleComponent`))
  (`self.CalculateHealth` Delta)
  (if (`self.isDead`)
    (bind _astwin_mode (cast `/Game/Blueprints/TwinMode` (`GameplayStatics.GetGameMode`)))
    (`/Game/Blueprints/TwinMode.Increment Score` _astwin_mode (`self.Score `))
    (`PrimitiveComponent.SetCollisionResponseToChannel` _capsulecomponent "ECC_WorldDynamic" "ECR_Ignore")
    (`PrimitiveComponent.SetCollisionResponseToChannel` _capsulecomponent "ECC_Pawn" "ECR_Ignore")
    (`self.DetachFromControllerPendingDestroy`)
    (`KismetSystemLibrary.Delay` 2.0)
    (`self.K2_DestroyActor`)))

(fn `UserConstructionScript`
  (bind _returnvalue (`PrimitiveComponent.CreateDynamicMaterialInstance` (`self.Mesh`) 0 null "None"))
  (bind _output_get (set `self.Dynamat` _returnvalue))
  (`MaterialInstanceDynamic.SetVectorParameterValue` _output_get "BodyColor" (`self.EnemyColor`)))