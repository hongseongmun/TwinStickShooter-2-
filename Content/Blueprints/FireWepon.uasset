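; FireWepon is a weapon Blueprint that spawns projectiles from three spawn points when its trigger is pulled.
; PullTrigger passes a DoOnce, fires the three SecondFire events once, then loops a timer on "Fire", a function not defined here, at RoundsPerSecond.
; ReleaseTrigger clears that timer and resets the DoOnce.
; Only secondFire2 sets a spawn class, FireProjectile_3; the other two spawns show none.
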(event `self.PullTrigger`
  (`/Engine/EditorBlueprintResources/StandardMacros.DoOnce` false :!label _label
    (:`Completed`
      (`self.secondFire2`)
      (`self.secondFire1`)
      (`self.secondFire`)
      (`KismetSystemLibrary.K2_SetTimer` null "Fire" (/ 1.0 (`self.RoundsPerSecond`)) true))))

(event `self.ReleaseTrigger`
  (`KismetSystemLibrary.K2_ClearTimer` null "Fire")
  (goto _label :!via `Reset`))

(event `secondFire`
  (`|SpawnActorFromClass` "/Game/Blueprints/FireProjectile.FireProjectile_C" (`SceneComponent.K2_GetComponentToWorld` (`self.ProjectileSpawnPoint`)) "Undefined" "OverrideRootScale" null null))

(event `secondFire1`
  (`|SpawnActorFromClass` "/Game/Blueprints/FireProjectile_2.FireProjectile_2_C" (`SceneComponent.K2_GetComponentToWorld` (`self.ProjectileSpawnPoint1`)) "Undefined" "OverrideRootScale" null null))

(event `secondFire2`
  (`|SpawnActorFromClass` "/Game/Blueprints/FireProjectile_3.FireProjectile_3_C" (`SceneComponent.K2_GetComponentToWorld` (`self.ProjectileSpawnPoint2`)) "Undefined" "OverrideRootScale" null null))

(fn `UserConstructionScript`
  (`parent.UserConstructionScript`))