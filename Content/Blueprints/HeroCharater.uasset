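; Player character for a twin-stick shooter, handling movement, aiming, weapons, health and footprint spawning.
; BeginPlay registers its spawn transform with TwinMode, adds the HUD and equips from two child-actor guns, which the mouse wheel cycles.
; Look input past a deadzone sets control rotation and pulls the equipped Weapon's trigger.
; Sprint raises walk speed while Tick drains or regenerates stamina through delays; death disables input, then requests respawn and destroys the character.
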(event `self.ReceiveBeginPlay`
  (`|ExecutionSequence`
    (:`then_1`
      (bind _astwin_mode (cast `/Game/Blueprints/TwinMode` (`GameplayStatics.GetGameMode`)))
      (bind _output_get (set `self.Gamemode` _astwin_mode))
      (set `/Game/Blueprints/TwinMode.Set player Spawn Transform` (`self.GetTransform`) _output_get))
    (:`then_2`
      (bind _returnvalue (`|CreateWidget` "/Game/Blueprints/TwinStickHUD.TwinStickHUD_C"))
      (`UserWidget.AddToViewport` _returnvalue 0))
    (:`then_3`
      (bind _output_get_2 (set `self.GunInventory` (`|MakeArray` (`self.PrimaryGun`) (`self.FireGun`))))
      (`self.EquipGun` _output_get_2))))

(event `InputAxisKey|MouseWheelAxis`
  (params (AxisValue :type "Float (single-precision)"))
  (bind _returnvalue (+ (`self.CurrentlyEquipped`) (`KismetMathLibrary.FTrunc` AxisValue)))
  (if (`KismetArrayLibrary.Array_IsValidIndex` (`self.GunInventory`) _returnvalue)
    (set `self.CurrentlyEquipped` _returnvalue)
    (`self.EquipGun` (`self.GunInventory`))
    (elif (< _returnvalue 0)
      (set `self.CurrentlyEquipped` (`KismetArrayLibrary.Array_LastIndex` (`self.GunInventory`)))
      (`self.EquipGun` (`self.GunInventory`))
      (else
        (set `self.CurrentlyEquipped` 0)
        (`self.EquipGun` (`self.GunInventory`))))))

(event `InputAxis|LookUp`
  (params (AxisValue :type "Float (single-precision)"))
  ;[1 1 1] Rotation
  (bind _asweapon (cast `/Game/Blueprints/Weapon` (`ChildActorComponent.ChildActor` (`|GetArrayItem` (`self.GunInventory`) (`self.CurrentlyEquipped`))) :!label _label))
  (bind _returnvalue (`KismetMathLibrary.MakeVector` AxisValue (stale `InputAxis|LookRight` AxisValue)))
  (if (> (`KismetMathLibrary.VSize` _returnvalue) 0.25)
    (`Controller.SetControlRotation` (`self.GetController`) (`KismetMathLibrary.Conv_VectorToRotator` _returnvalue))
    (`/Game/Blueprints/Weapon.PullTrigger` _asweapon)
    (else
      (`/Game/Blueprints/Weapon.ReleaseTrigger` _asweapon))))

(event `InputAxis|MoveUp`
  (params (AxisValue :type "Float (single-precision)"))
  ;[1 1 1] MoveMent
  (if (not (`self.DisableMovement`))
    (`self.AddMovementInput` (`self.World Direction_1`) AxisValue)))

(event `InputAxis|LookRight`
  (params (AxisValue :type "Float (single-precision)"))
  ;[1 1 1] Rotation
  (goto _label))

(event `InputAction|Sprint`
  (params (Key :type "Key Structure"))
  (bind _charactermovement (`self.CharacterMovement`))
  ;[1 1 1] MoveMent
  (:`Pressed`
    (if (>= (`self.Stamina`) 0.0)
      (set `self.IsSprinting` true)
      (set `CharacterMovementComponent.MaxWalkSpeed` 800.0 _charactermovement)
      (else
        (set `self.IsSprinting` false :!label _label_2)
        (set `CharacterMovementComponent.MaxWalkSpeed` 600.0 _charactermovement))))
  (:`Released`
    (goto _label_2)))

(event `InputAxis|MoveRight`
  (params (AxisValue :type "Float (single-precision)"))
  ;[1 1 1] MoveMent
  (if (not (`self.DisableMovement`))
    (`self.AddMovementInput` (`self.World Direction_0`) AxisValue)))

(event `/Game/Blueprints/iDamageable.AffectHealth`
  (params (Delta :type "Float (double-precision)"))
  (`self.CalculateHealth` Delta)
  (`KismetSystemLibrary.PrintString` (`KismetStringLibrary.Conv_DoubleToString` (`self.Health`)))
  (if (`self.isDead`)
    (`self.DisableInput` null)
    (`KismetSystemLibrary.Delay` 3.0)
    (`/Game/Blueprints/TwinMode.RespawnPlayer` (`self.Gamemode`))
    (`self.K2_DestroyActor` (`self.Wepon`))
    (`self.K2_DestroyActor` self)))

(event `self.ReceiveTick`
  (params (DeltaSeconds :type "Float (single-precision)"))
  ;[1 1 1] isSprintCheck
  (`|ExecutionSequence`
    (:`then_0`
      (if (`self.IsSprinting`)
        (`KismetSystemLibrary.Delay` 0.2)
        (if (<= (`self.Stamina`) 0.0)
          (set `self.IsSprinting` false)
          (set `CharacterMovementComponent.MaxWalkSpeed` 600.0 (`self.CharacterMovement`))
          (else
            (bind _output_get (set `self.Stamina` (- (`self.Stamina`) 1.0)))
            (`KismetSystemLibrary.PrintString` (`KismetStringLibrary.Conv_IntToString` (`KismetMathLibrary.FTrunc` _output_get)) :!label _label_3)))
        (else
          (`KismetSystemLibrary.Delay` 0.2)
          (if (< (`self.Stamina`) (`self.MaxStamina`))
            (set `self.Stamina` (+ (`self.Stamina`) 1.0))
            (goto _label_3)))))))

(event `SpawnFootprint L`
  ;[1 1 1] Spawn Player Foot
  (`|SpawnActorFromClass` "/Game/FootStep_L_BP.FootStep_L_BP_C" (`KismetMathLibrary.MakeTransform` (`SceneComponent.K2_GetComponentLocation` (`self.Foot `)) (`self.K2_GetActorRotation`) (0.1 0.1 0.1)) "Undefined" "OverrideRootScale" null null))

(event `SpawnFootprint R`
  ;[1 1 1] Spawn Player Foot
  (`|SpawnActorFromClass` "/Game/FootStep_R_BP.FootStep_R_BP_C" (`KismetMathLibrary.MakeTransform` (`SceneComponent.K2_GetComponentLocation` (`self.Foot R`)) (`self.K2_GetActorRotation`) (0.1 0.1 0.1)) "Undefined" "OverrideRootScale" null null))

(fn `EquipGun`
  (params (Array :type "Array of ChildActorComponent Object Reference"))
  (bind _output (`|GetArrayItem` Array (`self.CurrentlyEquipped`)))
  (for _array_element Array
    (`SceneComponent.SetVisibility` _array_element false false))
  (`SceneComponent.SetVisibility` _output true false)
  (`SceneComponent.K2_AttachToComponent` _output (`self.GunPointMesh`) "GripPoint" "SnapToTarget" "SnapToTarget" "SnapToTarget" true))

(fn `UserConstructionScript`)