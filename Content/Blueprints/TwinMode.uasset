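; TwinMode holds game-level logic for enemy spawning, player respawning and scoring, likely as a game mode.
; On BeginPlay it finds the first EnemySpawner in the level and sets a looping timer that calls its SpawnEnemy function at a rate derived from EnemiesPerSecond.
; RespawnPlayer spawns a new HeroCharater at the stored spawn transform and has player controller 0 possess it, while IncrementScore adds a delta to Score.
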(event `self.ReceiveBeginPlay`
  (bind _outactors (`GameplayStatics.GetAllActorsOfClass` "/Game/Blueprints/EnemySpawner.EnemySpawner_C"))
  (bind _output_get (set `self.Spawner` (`|GetArrayItem` _outactors)))
  (`KismetSystemLibrary.K2_SetTimer` _output_get "SpawnEnemy" (/ 1.0 (`self.EnemiesPerSecond`)) true))

(event `RespawnPlayer`
  (bind _returnvalue (`|SpawnActorFromClass` "/Game/Blueprints/HeroCharater.HeroCharater_C" (`self.Set player Spawn Transform`) "Undefined" "OverrideRootScale" null null))
  (`Controller.Possess` (`GameplayStatics.GetPlayerController` 0) _returnvalue))

(event `Increment Score`
  (params (`Delta Score` :type Integer))
  (set `self.Score` (+ `Delta Score` (`self.Score`))))

(fn `UserConstructionScript`)